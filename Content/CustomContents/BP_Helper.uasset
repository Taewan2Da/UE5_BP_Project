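; BP_Helper is a collection of stateless math helper functions for offsetting positions and converting normals to rotations.
; Up and down functions shift a vector along world Z, while forward, backward, left and right functions offset it along the axes of a supplied rotation.
; ReverseNormal builds a rotator from a normal as X, then uses a delta rotator to flip it 180 degrees around X.
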(fn `MoveVectorBackward`
  (params (InVector :type "Vector Structure") (InRotation :type "Rotator Structure") (SubtractValue :type "Float (double-precision)"))
  (returns (ReturnValue :type "Vector Structure"))
  ;[1 1 1] 현재액터의 위치에서 뒷 방향으로 이동가능
  (return (- InVector (* (`KismetMathLibrary.GetForwardVector` InRotation) SubtractValue))))

(fn `MoveVectorDownward`
  (params (InVector :type "Vector Structure") (SubtractValue :type "Float (double-precision)"))
  (returns (ReturnValue :type "Vector Structure"))
  ;[1 1 1] 현재 좌표를 z축아래 방향으로 내려주는 함수
  (return (- InVector (`KismetMathLibrary.MakeVector` 0.0 0.0 SubtractValue))))

(fn `MoveVectorForward`
  (params (InVector :type "Vector Structure") (InRotation :type "Rotator Structure") (AddValue :type "Float (double-precision)"))
  (returns (ReturnValue :type "Vector Structure"))
  ;[1 1 1] 현재액터의 위치에서 앞 방향으로 이동가능
  (return (+ InVector (* (`KismetMathLibrary.GetForwardVector` InRotation) AddValue))))

(fn `MoveVectorLeft`
  (params (InVector :type "Vector Structure") (InRotation :type "Rotator Structure") (MoveValue :type "Float (double-precision)"))
  (returns (ReturnValue :type "Vector Structure"))
  ;[1 1 1] 현재액터의 위치에서 왼쪽 방향으로 이동가능
  (return (- InVector (* (`KismetMathLibrary.GetRightVector` InRotation) MoveValue))))

(fn `MoveVectorRight`
  (params (InVector :type "Vector Structure") (InRotation :type "Rotator Structure") (MoveValue :type "Float (double-precision)"))
  (returns (ReturnValue :type "Vector Structure"))
  ;[1 1 1] 현재액터의 위치에서 오른쪽 방향으로 이동가능
  (return (+ InVector (* (`KismetMathLibrary.GetRightVector` InRotation) MoveValue))))

(fn `MoveVectorUpward`
  (params (InVector :type "Vector Structure") (AddValue :type "Float (double-precision)"))
  (returns (ReturnValue :type "Vector Structure"))
  ;[1 1 1] 현재 벡터에서 z축으로 값을 더해주는 벡터 좌표를 z축 위쪽 방향으로 올려주는 함수
  (return (+ InVector (`KismetMathLibrary.MakeVector` 0.0 0.0 AddValue))))

(fn `ReverseNormal`
  (params (InNormal :type "Vector Structure"))
  (returns (ReturnValue :type "Rotator Structure"))
  ;[1 1 1] x축을 중심으로180도 회전
  (return (`KismetMathLibrary.NormalizedDeltaRotator` (`KismetMathLibrary.MakeRotFromX` InNormal) (struct :`Yaw` 180.0))))