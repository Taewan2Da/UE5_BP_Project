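; Anti-gravity zone actor that switches off gravity for whatever overlaps its Cube component.
; On begin overlap, Characters get a zero CharacterMovement gravity scale, while other actors have gravity disabled on the overlapping component.
; On end overlap, gravity is re-enabled for components, and Characters receive a hardcoded gravity scale rather than their previous one.
; The construction script sizes the Cube from the Scale variable.
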(event `self.Cube.OnComponentBeginOverlap`
  (params (OverlappedComponent :type "PrimitiveComponent Object Reference") (OtherActor :type "Actor Object Reference") (OtherComp :type "PrimitiveComponent Object Reference") (OtherBodyIndex :type Integer) (bFromSweep :type Boolean) (SweepResult :type "HitResult Structure (by ref)"))
  (bind `_as캐릭터` (cast `Character` OtherActor)
    (:`then`
      (set `CharacterMovementComponent.GravityScale` 0.0 (`Character.CharacterMovement` `_as캐릭터`)))
    (:`CastFailed`
      (`PrimitiveComponent.SetEnableGravity` OtherComp false))))

(event `self.Cube.OnComponentEndOverlap`
  (params (OverlappedComponent :type "PrimitiveComponent Object Reference") (OtherActor :type "Actor Object Reference") (OtherComp :type "PrimitiveComponent Object Reference") (OtherBodyIndex :type Integer))
  (bind `_as캐릭터` (cast `Character` OtherActor)
    (:`then`
      (set `CharacterMovementComponent.GravityScale` 1.75 (`Character.CharacterMovement` `_as캐릭터`)))
    (:`CastFailed`
      (`PrimitiveComponent.SetEnableGravity` OtherComp true))))

(fn `UserConstructionScript`
  (`SceneComponent.SetWorldScale3D` (`self.Cube`) (`self.Scale`)))